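; Competitive character Blueprint for UEtopia that shows an overhead widget and creates the local player's HUD.
; Every Tick it pushes Health to the widget's progress bar and copies the title from MyPlayerState into it.
; Tick also billboards the Scene component by yaw only toward player 0's camera.
; BeginPlay adds the HUD to the viewport only when locally controlled, otherwise printing a debug message.
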(event EventBeginPlay
  ;[1 1 1] Create HUD
  (if (Pawn|IsLocallyControlled self)
    (bind _returnvalue (UserInterface|CreateWidget "/Game/HUD.HUD_C" (Game|GetPlayerController 0)))
    (Utilities|IsValid _returnvalue
      (:Is%20Valid
        (UserInterface|Viewport|AddtoViewport _returnvalue 0)))
    (else
      (Development|PrintString "BeginPlay NOT Locally controlled"))))

(event Collision|EventActorBeginOverlap
  (params (OtherActor :type Actor%20Object%20Reference)))

(event EventTick
  (params (DeltaSeconds :type Float%20%28single-precision%29))
  (bind _scene (Variables|Default|GetScene))
  (bind _asplayer_overhead (Utilities|Casting|CastToPlayerOverhead (UserInterface|GetUserWidgetObject (Variables|Default|GetWidget))))
  (Progress|SetPercent (Variables|/Game/UI/PlayerOverhead.PlayerOverhead_C|GetProgressBar_96 _asplayer_overhead) (Variables|Default|GetHealth))
  (Transformation|SetWorldRotation _scene (Math|Rotator|MakeRotator 0.0 0.0 (.Yaw (Math|Rotator|BreakRotator (Math|Rotator|FindLookatRotation (Transformation|GetWorldLocation _scene) (Transformation|GetActorLocation (Game|GetPlayerCameraManager 0)))))) false false)
  ;[1 1 1] Set Player Title
  (bind _asmy_player_state (Utilities|Casting|CastToMyPlayerState (Variables|Default|GetPlayerState)))
  (bind _asplayer_overhead_2 (Utilities|Casting|CastToPlayerOverhead (UserInterface|GetUserWidgetObject (Variables|Default|GetWidget))))
  (Rendering|Components|TextRender|SetText (Variables|/Game/UI/PlayerOverhead.PlayerOverhead_C|GetPlayerTitle _asplayer_overhead_2) (Utilities|Text|ToText(String) (Variables|/Script/ProESports.MyPlayerState|GetplayerTitle _asmy_player_state))))

(fn ConstructionScript)